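; Item chest interactable that opens only for a pawn carrying a required key.
; Interact checks the instigator's SActionComponent active gameplay tags for RequiredKey before calling the parent Interact.
; InteractAnimation plays or reverses a Timeline from LidOpened to pitch the lid mesh, and GetInteractText returns the Tips text.
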(event `self.InteractAnimation`
  (if (`self.bLidOpened`)
    (bind (_direction _newtrack_1) (`Timeline|Timeline` :!label _label)
      (:`Update`
        (`SceneComponent.K2_SetRelativeRotation` (`self.LidMesh`) (`KismetMathLibrary.MakeRotator` 0.0 _newtrack_1) false false)))
    (else
      (goto _label :!via `Reverse`))))

(event `SGameplayInterface.Interact`
  (params (InstigatorPawn :type "Pawn Object Reference"))
  (if (`BlueprintGameplayTagLibrary.HasTag` (`SActionComponent.ActiveGameplayTags` (`self.GetComponentByClass` InstigatorPawn "/Script/SGames.SActionComponent")) (`self.RequiredKey`))
    (`parent.Interact` InstigatorPawn)))

(fn `GetInteractText`
  (params (InstigatorPawn :type "Pawn Object Reference"))
  (returns (ReturnValue :type Text))
  (return (`self.Tips`)))

(fn `UserConstructionScript`)